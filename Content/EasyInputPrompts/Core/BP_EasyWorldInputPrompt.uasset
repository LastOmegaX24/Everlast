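; BP_EasyWorldInputPrompt places an input prompt in the world through a widget component, with configurable display space, keys or input action, text and styling.
; On BeginPlay it passes its settings to the WBP_EasyMultiInputPromptDisplayer inside that component.
; For adjustable resolution, CalculateFinalResolution supplies icon size and font scaled by ResolutionMultiplier, then UpdateWidgetScale divides the component's world scale by the same factor.
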(event EventBeginPlay
  (bind (_returnvalue _textfont) (|CalculateFinalResolution))
  (bind _aswbp_easy_multi_input_prompt_displayer (Utilities|Casting|CastToWBP_EasyMultiInputPromptDisplayer (UserInterface|GetWidget (Variables|Default|GetWidget))))
  (Default|SetupWidget _aswbp_easy_multi_input_prompt_displayer (Variables|EasyConfig|Keys|GetUse%20Input%20Action?) (Variables|EasyConfig|Keys|GetInput%20Action) (Variables|EasyConfig|Keys|GetInput%20Mapping%20Context) (Variables|EasyConfig|Keys|GetGamepad%20Keys) (Variables|EasyConfig|Keys|GetMNK%20Keys) _returnvalue (Variables|EasyConfig|Styling|GetText%20To%20Display) _textfont (Variables|EasyConfig|Styling|GetText%20Position) (Variables|EasyConfig|Styling|GetText%20Padding) (Variables|EasyConfig|Styling|GetText%20Transform%20Policy) (Variables|EasyConfig|Styling|GetText%20Justification) (Variables|EasyConfig|Styling|GetSpacing) (Variables|EasyConfig|Styling|GetText%20Color) (Variables|EasyConfig|Styling|GetIcon%20Color) (Variables|EasyConfig|Keys|GetHide%20Key%20For%20Other%20Devices?) (Variables|EasyConfig|Keys|GetHideTextAsWell?))
  (|UpdateWidgetScale))

(fn ConstructionScript
  (Class|WidgetComponent|SetWidgetSpace (Variables|Default|GetWidget) (Variables|EasyConfig|Styling|GetDisplayType)))