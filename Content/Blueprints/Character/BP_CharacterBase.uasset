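; Base character for turn-based combat that handles abilities, attacks, health and damage feedback.
; BeginPlay grants the ability list; a basic attack checks turn and usability, then ends the turn as a timeline-driven arc jump carries the character to the target's front.
; On landing it activates the first GAS ability and hops back after a delay.
; Damage spawns numbers and ragdolls at zero health; skill and ultimate events are empty stubs.
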(event Custom|BasicAttack
  (params (target :type BP%20Character%20Base%20Object%20Reference))
  (Utilities|Array|Clear (Variables|Default|GetTarget_Arr))
  (Utilities|CanUseSkill
    (:True
      (CallFunction|Jumpto (Transformation|GetActorLocation) (Transformation|GetWorldLocation (Variables|BP_CharacterBase_C|GetFrontTarget target)) false 1e+02)
      (Utilities|Array|Add (Variables|Default|GetTarget_Arr) target)
      (Default|EndTurn (Variables|Default|GetCombatComponent)))))

(event Custom|Skill_A)

(event Custom|Skill_B)

(event Custom|Skill_C)

(event Custom|Ultimate)

(event Custom|JumpTo
  (params (Start :type Vector) (Target :type Vector) (Return :type Boolean) (Height :type Float%20%28double-precision%29))
  (bind (_direction _location _jump) (Timeline|JumpToTarget PlayFromStart)
    (:Update
      (Transformation|SetActorLocation (+ (Math|Vector|Lerp(Vector) Start Target _location) (Math|Vector|MakeVector 0.0 0.0 (* _jump Height))) false false))
    (:Finished
      (if (not Return)
        (CallFunction|AfterJumptoFinished)))))

(event Custom|AfterJumpToFinished
  (bind _returnvalue (Class|AbilitySystemComponent|TryActivateAbility (Variables|Default|GetAbilitySystem) (Utilities|Array|Get(acopy) (Variables|Default|GetAbilityList)) true))
  (if _returnvalue
    _
    (else
      _))
  (Utilities|FlowControl|Delay 1.0)
  (CallFunction|Jumpto (Transformation|GetActorLocation) (Variables|Default|GetStartLocation) true 1e+02))

(event Custom|DamageNumbers
  (params (Damage :type Float%20%28double-precision%29))
  (Game|SpawnActorfromClass "/Game/UI/DamageNumActor.DamageNumActor_C" (Transformation|GetActorTransform) "Undefined" "MultiplyWithRoot" 0 Damage 0))

(event Custom|Heal
  (params (Amount :type Float%20%28double-precision%29) (Overheal :type Boolean))
  (Variables|Default|SetHealth (Math|Float|SelectFloat (+ (Variables|Default|GetHealth) Amount) (Math|Float|Clamp(Float) (+ (Variables|Default|GetHealth) Amount) 0.0 (Variables|Default|GetMaxHealth)) Overheal)))

(event Game|Damage|EventAnyDamage
  (params (Damage :type Float%20%28single-precision%29) (DamageType :type Damage%20Type%20Object%20Reference) (InstigatedBy :type Controller%20Object%20Reference) (DamageCauser :type Actor%20Object%20Reference))
  (Variables|Default|SetHealth (- (Variables|Default|GetHealth) Damage))
  (if (> Damage 0.0)
    (CallFunction|DamageNumbers Damage)
    (if (<= (Variables|Default|GetHealth) 0.0)
      (Physics|SetSimulatePhysics (Variables|Default|GetSkeletalMesh) true))))

(event EventBeginPlay
  (Variables|Default|SetStartLocation (Transformation|GetActorLocation))
  (for (_array_element _array_index) (Variables|Default|GetAbility%20Class)
    (bind _returnvalue (GameplayAbilities|GiveAbility (Variables|Default|GetAbilitySystem) _array_element 0 _array_index))
    (Utilities|Array|Add (Variables|Default|GetAbilityList) _returnvalue)))

(fn ConstructionScript)