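; Test character Blueprint that triggers an ability as a turn-based combat action.
; The SkillA event runs through the CanUseSkill macro, which passes only when CombatComponent reports its turn and CanUseAbility is set.
; On success it asks the AbilitySystem to activate the second AbilityList entry, then ends the turn on CombatComponent without checking the activation result.
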(event EventSkillA
  (Utilities|CanUseSkill
    (:True
      (Class|AbilitySystemComponent|TryActivateAbility (Variables|Default|GetAbilitySystem) (Utilities|Array|Get(acopy) (Variables|Default|GetAbilityList) 1) true)
      (Default|EndTurn (Variables|Default|GetCombatComponent)))))

(fn ConstructionScript
  (|CallParentFunction))