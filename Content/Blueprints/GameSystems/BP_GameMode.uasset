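; BP_GameMode is a game mode Blueprint with hooks for team- and turn-based play.
; On BeginPlay it spawns an AI_Camera actor, and its EndTurn event calls ResetTurnForAll on the player passed in.
; GetCharacters branches by team, with the default sharing team 0's path, but it and GetSpawnedActors show no returned data.
; GetIsTurn always returns false.
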(event EventBeginPlay
  (Game|SpawnActorfromClass "/Game/Blueprints/GameSystems/Game/AI_Camera.AI_Camera_C" (Math|Transform|MakeTransform "0, 0, 0" "0, 0, 0" "1.000000,1.000000,1.000000") "Undefined" "MultiplyWithRoot" 0 0))

(event EventEndTurn
  (params (PlayerToEndTurn :type Game%20Third%20Person%20Camera%20Object%20Reference))
  (Default|ResetTurnforAll PlayerToEndTurn))

(fn ConstructionScript)

(fn GetSpawnedActors
  (return 0))

(fn GetCharacters
  (params (Team :type Integer))
  (switch int Team
    (:Default
      _)
    (:0
      _)
    (:1
      (return 0))
    (:2
      (return 0)))
  (return 0))

(fn GetIsTurn
  (params (Team :type Integer))
  (return false))